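; Player character Blueprint with movement along the world X axis, featuring double jump, wall jump and air dash.
; On jump, a line trace from behind to ahead of the capsule detects walls and launches the character away from any hit.
; Otherwise it jumps or relaunches upward in midair, using a counter that resets on landing.
; Dash works only while falling, launching along the last input direction while keeping vertical velocity.
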(event `self.OnLanded`
  (params (Hit :type "HitResult Structure (by ref)"))
  (set `self.jumpTimes` 0))

(event `InputAxis|Move`
  (params (AxisValue :type "Float (single-precision)"))
  (`self.AddMovementInput` (1.0 0.0 0.0) AxisValue)
  (set `self.direction_requested` AxisValue))

(event `InputAction|Jump`
  (params (Key :type "Key Structure"))
  (bind _returnvalue_x (`KismetMathLibrary.BreakVector` (`self.K2_GetActorLocation`)))
  (bind _returnvalue (`self.K2_GetActorLocation`))
  (bind _charactermovement (`self.CharacterMovement`))
  (bind _returnvalue_2 (* (`self.GetActorForwardVector`) (+ (`CapsuleComponent.GetScaledCapsuleRadius` (`self.CapsuleComponent`)) 16.0)))
  (:`Pressed`
    (bind (_outhit _returnvalue_3) (`KismetSystemLibrary.LineTraceSingle` (- _returnvalue _returnvalue_2) (+ _returnvalue _returnvalue_2) "TraceTypeQuery1" true))
    (if _returnvalue_3
      (`self.LaunchCharacter` (`KismetMathLibrary.MakeVector` (* (`KismetMathLibrary.SignOfFloat` (- _returnvalue_x (.x (`.Location` (`GameplayStatics.BreakHitResult` _outhit))))) 450.0) 0.0 (`CharacterMovementComponent.JumpZVelocity` _charactermovement)) true true)
      (elif (< (`self.jumpTimes`) 2)
        (if (`NavMovementComponent.IsFalling` _charactermovement)
          (`self.LaunchCharacter` (0.0 0.0 400.0) false true)
          (else
            (`self.Jump`)))
        (set `self.jumpTimes` (+ (`self.jumpTimes`) 1)))))
  (:`Released`
    (`self.StopJumping`)))

(event `InputAction|Dash`
  (params (Key :type "Key Structure"))
  (bind _charactermovement (`self.CharacterMovement`))
  (bind (_velocity_x _velocity_y _velocity_z) (`KismetMathLibrary.BreakVector` (`MovementComponent.Velocity` _charactermovement)))
  (:`Pressed`
    (if (`NavMovementComponent.IsFalling` _charactermovement)
      (`self.LaunchCharacter` (`KismetMathLibrary.MakeVector` (* (`self.direction_requested`) 500.0) 0.0 _velocity_z) true true))))

(fn `UserConstructionScript`
  (set `CharacterMovementComponent.JumpZVelocity` 400.0 (`self.CharacterMovement`))
  (set `self.JumpMaxHoldTime` 0.3))